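; Game mode for the first level that runs a countdown and ends play when time runs out.
; A looping one-second timer, started on BeginPlay, decrements GameTime.
; At exactly zero, if OnPause is not already set, it pauses the game, shows the W_TimeOut widget, switches to UI-only input with a visible cursor and clears the timer.
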(event `self.ReceiveBeginPlay`
  (bind _returnvalue (`KismetSystemLibrary.K2_SetTimerDelegate` (delegate `CustomEvent`) 1.0 true))
  (set `self.GameTimerHandle` _returnvalue))

(event `CustomEvent`
  (bind _output_get (set `self.GameTime` (- (`self.GameTime`) 1)))
  (if (== _output_get 0)
    (if (not (`self.OnPause`))
      (set `self.OnPause` true)
      (`GameplayStatics.SetGamePaused` true)
      (bind _returnvalue (`|CreateWidget` "/Game/LMA/UI/W_TimeOut.W_TimeOut_C"))
      (bind _output_get_2 (set `self.W_Time_Out_Widget` _returnvalue))
      (`UserWidget.AddToViewport` _output_get_2 0)
      (`WidgetBlueprintLibrary.SetInputMode_UIOnlyEx` (`GameplayStatics.GetPlayerController` 0) null)
      (set `PlayerController.bShowMouseCursor` true (`GameplayStatics.GetPlayerController` 0))
      (`KismetSystemLibrary.K2_ClearAndInvalidateTimerHandle` (`self.GameTimerHandle`)))))

(fn `UserConstructionScript`)